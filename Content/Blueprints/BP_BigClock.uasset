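; BP_BigClock is a VR puzzle clock whose hands advance one step per interaction to match an externally set target time.
; Right-controller overlap on the hour or minute collider selects the hand, with hour changes gated by HoursEnabled.
; A matching time triggers OnSpawnBooks on every BP_Book, once only.
; A separate OpenDoor event enables the first BP_Key and swings the clock door open via timeline.
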(event OnComponentBeginOverlap(HourColl)
  (params (OverlappedComponent :type Primitive%20Component%20Object%20Reference) (OtherActor :type Actor%20Object%20Reference) (OtherComp :type Primitive%20Component%20Object%20Reference) (OtherBodyIndex :type Integer) (bFromSweep :type Boolean) (SweepResult :type Hit%20Result%20Structure%20%28by%20ref%29))
  ;[1 1 1] Check if Controller overlaps Minute or Hour Button
  (bind _outactors (Actor|GetAllActorsOfClass "/Game/VirtualRealityBP/Blueprints/MotionControllerPawn.MotionControllerPawn_C"))
  (if (== (Variables|/Game/VirtualRealityBP/Blueprints/MotionControllerPawn.MotionControllerPawn_C|GetRightController (Utilities|Array|Get(acopy) _outactors)) OtherActor)
    (Variables|Default|SetHourMinuteButton "Hour")))

(event OnComponentBeginOverlap(MinuteColl)
  (params (OverlappedComponent :type Primitive%20Component%20Object%20Reference) (OtherActor :type Actor%20Object%20Reference) (OtherComp :type Primitive%20Component%20Object%20Reference) (OtherBodyIndex :type Integer) (bFromSweep :type Boolean) (SweepResult :type Hit%20Result%20Structure%20%28by%20ref%29))
  ;[1 1 1] Check if Controller overlaps Minute or Hour Button
  (bind _outactors (Actor|GetAllActorsOfClass "/Game/VirtualRealityBP/Blueprints/MotionControllerPawn.MotionControllerPawn_C"))
  (if (== (Variables|/Game/VirtualRealityBP/Blueprints/MotionControllerPawn.MotionControllerPawn_C|GetRightController (Utilities|Array|Get(acopy) _outactors)) OtherActor)
    (Variables|Default|SetHourMinuteButton "Minute")))

(event Custom|SetNeededHour
  (params (Hour :type String))
  (Variables|Default|SetNeededHour Hour))

(event Custom|SetNeededMinute
  (params (Minute :type String))
  (Variables|Default|SetNeededMinute Minute))

(event Custom|OpenDoor
  (bind _outactors (Actor|GetAllActorsOfClass "/Game/Blueprints/BP_Key.BP_Key_C"))
  (Default|EnableKey (Utilities|Array|Get(acopy) _outactors))
  (bind _clockdoortrack (Timeline|OpenClockDoor PlayFromStart)
    (:Update
      (Transformation|SetWorldRotation (Variables|Default|GetDoor) (Math|Rotator|MakeRotator 0.0 0.0 _clockdoortrack) false false))))

(event EventInteract
  (switch string (Variables|Default|GetHourMinuteButton)
    (:Minute
      (bind _output_get (Variables|Default|SetCurrentMinute (+ (Variables|Default|GetCurrentMinute) 1)))
      (Utilities|FlowControl|Sequence
        (:then_0
          (if (>= _output_get 60)
            (Variables|Default|SetCurrentMinute 0)))
        (:then_1
          (Transformation|AddLocalRotation (Variables|Default|GetMinutePointer) "0.0,6.000000,0.000000" false false)
          (if (and (Utilities|Enum|Equal(Enum) (Variables|Default|GetNeededMinute) (Utilities|String|ToString(Integer) (Variables|Default|GetCurrentMinute))) (Utilities|Enum|Equal(Enum) (Variables|Default|GetNeededHour) (Utilities|String|ToString(Integer) (Variables|Default|GetCurrentHour)))) :!label _label
            (Development|PrintString "a7")
            (if (Variables|Default|GetSpawnedBooks)
              (Development|PrintString "c7")
              (else
                (Development|PrintString "d7")
                (Variables|Default|SetSpawnedBooks true)
                (bind _outactors (Actor|GetAllActorsOfClass "/Game/Blueprints/BP_Book.BP_Book_C"))
                (Development|PrintString (Utilities|String|Append (Utilities|String|ToString(Integer) (Utilities|Array|Length _outactors)) "books found"))
                (for _array_element _outactors
                  (Default|OnSpawnBooks _array_element))))))))
    (:Hour
      (if (Variables|Default|GetHoursEnabled)
        (bind _output_get_2 (Variables|Default|SetCurrentHour (+ (Variables|Default|GetCurrentHour) 1)))
        (Utilities|FlowControl|Sequence
          (:then_0
            (if (>= _output_get_2 12)
              (Variables|Default|SetCurrentHour 0)))
          (:then_1
            (Transformation|AddLocalRotation (Variables|Default|GetHourPointer) "0,30.000000,0.000000" false false)
            (goto _label)))))))

(fn ConstructionScript)