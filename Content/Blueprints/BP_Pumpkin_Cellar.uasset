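; BP_Pumpkin_Cellar is a pumpkin prop that a motion controller can pick up and that displays part of a code.
; SetText splits the code on semicolons and shows the second segment, wrapped in underscores, on its text render.
; Pickup turns off the pumpkin's physics and attaches the root to the supplied component; Drop restores physics and detaches the actor, both keeping world transforms.
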(event Custom|Set%20Text
  (params (Code :type String))
  (Rendering|Components|TextRender|SetText (Variables|Default|GetTextRender) (Utilities|Text|ToText(String) (Utilities|String|Append "_" (Utilities|Array|Get(acopy) (Utilities|String|ParseIntoArray Code ";") 1) "_"))))

(event EventPickup
  (params (AttachTo :type Scene%20Component%20Object%20Reference))
  (Physics|SetSimulatePhysics (Variables|Default|GetPumpkin) false)
  (Transformation|AttachComponentToComponent (VehicleSound|GetRootComponent) AttachTo "None" "KeepWorld" "KeepWorld" "KeepWorld" false))

(event EventDrop
  (Physics|SetSimulatePhysics (Variables|Default|GetPumpkin) true)
  (Transformation|DetachFromActor "KeepWorld" "KeepWorld" "KeepWorld"))

(fn ConstructionScript)