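; BP_LightController makes three point lights flicker in bursts that signal an hour number, repeating until the count is read.
; SetHours stores the count, and EnableFlickering replays the LightFlickerOnce timeline that many times, setting all three intensities from MaxIntensity and the truncated curve multiplier.
; The WaitForSeconds timeline provides the pause between bursts, then the counter resets and the cycle loops indefinitely.
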(event Custom|Enable%20Flickering
  ;[1 1 1] Flicker the ammount of times that equals the hour it needs to be on
  (bind _intensitymultiplier (Timeline|LightFlickerOnce PlayFromStart)
    (:Update
      (Rendering|Components|Light|SetIntensity (Variables|Default|GetPointLight) (Math|Conversions|ToFloat(Integer) (* (Variables|Default|GetMaxIntensity) (Math|Float|Truncate _intensitymultiplier))))
      (Rendering|Components|Light|SetIntensity (Variables|Default|GetPointLight1) (Math|Conversions|ToFloat(Integer) (* (Variables|Default|GetMaxIntensity) (Math|Float|Truncate _intensitymultiplier))))
      (Rendering|Components|Light|SetIntensity (Variables|Default|GetPointLight2) (Math|Conversions|ToFloat(Integer) (* (Variables|Default|GetMaxIntensity) (Math|Float|Truncate _intensitymultiplier)))))
    (:Finished
      (Variables|Default|SetCurrent%20Flicker (- (Variables|Default|GetCurrent%20Flicker) 1))
      (if (<= (Variables|Default|GetCurrent%20Flicker) 0)
        ;[1 1 1] Waits before next flicker
        (Timeline|WaitForSeconds PlayFromStart
          (:Finished
            (Variables|Default|SetCurrent%20Flicker (Variables|Default|GetNumber))
            (CallFunction|EnableFlickering)))
        (else
          (Timeline|LightFlickerOnce PlayFromStart))))))

(event Custom|Set%20Hours
  (params (Number :type Integer))
  ;[1 1 1] Sets FlickerNumber based on needed Hours
  (bind _output_get (Variables|Default|SetNumber Number))
  (Variables|Default|SetCurrent%20Flicker _output_get))

(fn ConstructionScript)