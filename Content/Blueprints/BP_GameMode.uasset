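; Game mode that generates and validates randomized puzzle codes for the cellar door, safe and clock.
; On BeginPlay it rolls three-digit cellar and safe codes plus an hour and minute, then passes the time to the light controller, big clock and painting.
; Match events count entries for the cellar and safe, compare the entered string after three, and either set the open flag or reset the attempt.
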(event Custom|Match_Code_Cellar
  (Math|Integer|IncrementInt (Variables|Count|GetCellCount)
    (:%20%20
      (if (>= (Variables|Count|GetCellCount) 3)
        (if (Utilities|Enum|Equal(Enum) (Variables|RandomFinalCode|GetDoorCellarCode) (Variables|ActuallyCode|GetActualCellDoorCode))
          (Variables|OpenBool|SetCellDoorOpen true)
          (else
            (Variables|Count|SetCellCount 0)
            (Variables|ActuallyCode|SetActualCellDoorCode "")))))))

(event Custom|Match_Code_Safe
  (Math|Integer|IncrementInt (Variables|Count|GetSafeCount)
    (:%20%20
      (if (>= (Variables|Count|GetSafeCount) 3)
        (if (Utilities|Enum|Equal(Enum) (Variables|RandomFinalCode|GetSafeCode) (Variables|ActuallyCode|GetActualSafeCode))
          (Variables|OpenBool|SetSafeOpen true)
          (else
            (Variables|Count|SetSafeCount 0)
            (Variables|ActuallyCode|SetActualSafeCode "")))))))

(event EventBeginPlay
  (bind _returnvalue (Math|Random|RandomIntegerinRange 100 999))
  (bind _returnvalue_2 (Utilities|String|ToString(Integer) _returnvalue))
  (Variables|RandomFinalCode|SetDoorCellarCode _returnvalue_2)
  (Variables|RandomFinalCode|SetSafeCode _returnvalue_2)
  (Variables|RandomFinalCode|SetHourCode (Utilities|String|ToString(Integer) (Math|Random|RandomIntegerinRange 1 12)))
  (Variables|RandomFinalCode|SetMinuteCode (Utilities|String|ToString(Integer) (Math|Random|RandomIntegerinRange 0 59)))
  ;[1 1 1] Set Hour and Minute Values in Clock, Painting, Lights
  (bind _outactors (Actor|GetAllActorsOfClass "/Game/Blueprints/BP_LightController.BP_LightController_C"))
  (Default|SetHours (Utilities|Array|Get(acopy) _outactors) (Math|Conversions|ToInteger(Byte) (Variables|RandomFinalCode|GetHourCode)))
  (bind _outactors_2 (Actor|GetAllActorsOfClass "/Game/Blueprints/BP_BigClock.BP_BigClock_C"))
  (Default|SetNeededHour (Utilities|Array|Get(acopy) _outactors_2) (Variables|RandomFinalCode|GetHourCode))
  (Default|SetNeededMinute (Utilities|Array|Get(acopy) _outactors_2) (Variables|RandomFinalCode|GetMinuteCode))
  (bind _outactors_3 (Actor|GetAllActorsOfClass "/Game/Blueprints/BP_Painting.BP_Painting_C"))
  (Default|SetMinute (Utilities|Array|Get(acopy) _outactors_3) (Variables|RandomFinalCode|GetMinuteCode)))

(fn ConstructionScript)