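; BP_Safe is a safe that shows a code on its text render and, when opened, reveals part of the cellar door code.
; OpenSafe destroys every BP_ButtonTresor in the world, then spawns a small number actor at the Spawn point, passing it the second segment of the GameMode's semicolon-separated code.
; The SafeOpener timeline then drives the door's absolute world yaw; the saved StartRotation is not used in the swing.
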(event Custom|SetText
  (params (ActualCode :type String))
  (Rendering|Components|TextRender|SetText (Variables|Default|GetTextRender) (Utilities|Text|ToText(String) ActualCode)))

(event Custom|Open%20Safe
  (Variables|Default|SetStartRotation (.yaw (Transformation|GetWorldRotation (Variables|Default|GetDoor))))
  (bind _outactors (Actor|GetAllActorsOfClass "/Game/Blueprints/BP_ButtonTresor.BP_ButtonTresor_C"))
  (for _array_element _outactors
    (Actor|DestroyActor _array_element))
  (bind _returnvalue (Game|SpawnActorfromClass "/Game/Blueprints/BP_Nummerzweiplceholder.BP_Nummerzweiplceholder_C" (Math|Transform|MakeTransform (Transformation|GetWorldLocation (Variables|Default|GetSpawn)) "0, 0, 0" "0.100000,0.100000,0.100000") "Undefined" 0 0))
  (Default|Zahl _returnvalue (Utilities|Array|Get(acopy) (Utilities|String|ParseIntoArray (Variables|/Game/Blueprints/BP_GameMode.BP_GameMode_C|GetDoorCellarCodeParser (Variables|Default|GetGamemode)) ";") 1))
  (bind _safe (Timeline|Safe%20Opener PlayFromStart)
    (:Update
      (Transformation|SetWorldRotation (Variables|Default|GetDoor) (Math|Rotator|MakeRotator 0.0 0.0 _safe) false false))))

(event EventBeginPlay
  (bind _asbp_game_mode (Utilities|Casting|CastToBP_GameMode (Game|GetGameMode)))
  (Variables|Default|SetGamemode _asbp_game_mode))

(fn ConstructionScript)