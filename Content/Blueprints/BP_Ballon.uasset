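; A VR balloon actor that floats and can be grabbed by motion controllers.
; Each tick it applies a tiny upward force to the Ballon component.
; Pickup, called by BP_MotionController, disables physics and attaches the root to the given component, keeping world transform.
; Drop re-enables physics and detaches the actor.
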(event EventPickup
  (params (AttachTo :type Scene%20Component%20Object%20Reference))
  (Physics|SetSimulatePhysics (Variables|Default|GetBallon) false)
  (Transformation|AttachComponentToComponent (VehicleSound|GetRootComponent) AttachTo "None" "KeepWorld" "KeepWorld" "KeepWorld" false))

(event EventTick
  (params (DeltaSeconds :type Float%20%28single-precision%29))
  (Physics|AddForce (Variables|Default|GetBallon) "0, 0,0.001000" "None" false))

(event EventDrop
  (Physics|SetSimulatePhysics (Variables|Default|GetBallon) true)
  (Transformation|DetachFromActor "KeepWorld" "KeepWorld" "KeepWorld"))

(fn ConstructionScript)