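; BP_TV is a one-shot scare prop that, on Interact, reveals a head mesh yawed toward the MotionControllerPawn with a fixed offset.
; SpookyTimeline times the scare, and its first update plays a 2D white noise sound that stops after a delay.
; When the timeline finishes, it hides the head, enables flickering on BP_LightController and sets HoursEnabled on BP_BigClock, finding both by class lookup.
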(event EventBeginPlay)

(event Collision|EventActorBeginOverlap
  (params (OtherActor :type Actor%20Object%20Reference)))

(event EventTick
  (params (DeltaSeconds :type Float%20%28single-precision%29)))

(event EventInteract
  (bind _headmesh (Variables|Default|GetHeadMesh))
  ;[1 1 1] Show Ghost, Play Sound, make Light flickering
  (if (not (Variables|Default|GetWasActivated))
    (Variables|Default|SetWasActivated true)
    (Rendering|SetVisibility _headmesh true false)
    (bind _outactors (Actor|GetAllActorsOfClass "/Game/VirtualRealityBP/Blueprints/MotionControllerPawn.MotionControllerPawn_C"))
    (Transformation|SetRelativeRotation _headmesh (Math|Rotator|MakeRotator 0.0 0.0 (- (.yaw (Math|Rotator|FindLookatRotation (.location (Transformation|GetWorldTransform _headmesh)) (Transformation|GetActorLocation (Utilities|Array|Get(acopy) _outactors)))) 2e+01)) false false)
    (Timeline|SpookyTimeline PlayFromStart
      (:Update
        (if (not (Variables|Default|GetSoundPlayed))
          (Variables|Default|SetSoundPlayed true)
          (bind _returnvalue (Audio|SpawnSound2D "/Game/Audio/Sound_WhiteNoise.Sound_WhiteNoise" 1.0 1.0 0.0 0))
          (Utilities|FlowControl|Delay 5.0)
          (Audio|Components|Audio|Stop _returnvalue)))
      (:Finished
        (Rendering|SetVisibility (Variables|Default|GetHeadMesh) false false)
        (bind _outactors_2 (Actor|GetAllActorsOfClass "/Game/Blueprints/BP_LightController.BP_LightController_C"))
        (Default|EnableFlickering (Utilities|Array|Get(acopy) _outactors_2))
        (bind _outactors_3 (Actor|GetAllActorsOfClass "/Game/Blueprints/BP_BigClock.BP_BigClock_C"))
        (Variables|/Game/Blueprints/BP_BigClock.BP_BigClock_C|SetHoursEnabled (Utilities|Array|Get(acopy) _outactors_3) true)))))

(fn ConstructionScript)