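; BP_Paper_Safe is a grabbable VR paper clue that reveals part of the cellar door code.
; On BeginPlay it splits the code string from BP_GameMode on semicolons and displays the third entry behind two underscore placeholders on its text render.
; Pickup, called by BP_MotionController, disables the paper's physics and attaches it to the given component; Drop re-enables physics and detaches it.
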(event EventPickup
  (params (AttachTo :type Scene%20Component%20Object%20Reference))
  (Physics|SetSimulatePhysics (Variables|Default|GetPaper) false)
  (Transformation|AttachComponentToComponent (VehicleSound|GetRootComponent) AttachTo "None" "KeepWorld" "KeepWorld" "KeepWorld" false))

(event EventBeginPlay
  (bind _asbp_game_mode (Utilities|Casting|CastToBP_GameMode (Game|GetGameMode)))
  (Rendering|Components|TextRender|SetText (Variables|Default|GetTextRender) (Utilities|Text|ToText(String) (Utilities|String|Append "_" "_" (Utilities|Array|Get(acopy) (Utilities|String|ParseIntoArray (Variables|/Game/Blueprints/BP_GameMode.BP_GameMode_C|GetDoorCellarCodeParser _asbp_game_mode) ";") 2)))))

(event EventDrop
  (Physics|SetSimulatePhysics (Variables|Default|GetPaper) true)
  (Transformation|DetachFromActor "KeepWorld" "KeepWorld" "KeepWorld"))

(fn ConstructionScript)