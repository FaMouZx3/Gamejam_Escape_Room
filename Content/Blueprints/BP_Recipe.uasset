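; BP_Recipe is a recipe object that the player picks up and drops with a motion controller.
; Pickup, called by BP_MotionController, turns off physics on its Box and attaches the root to the given component, keeping world transform.
; Drop re-enables physics and detaches the actor.
; BeginPlay stores the Recipe component's world location, which these graphs do not use further.
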(event EventBeginPlay
  (Variables|Default|SetLocation (Transformation|GetWorldLocation (Variables|Default|GetRecipe))))

(event EventPickup
  (params (AttachTo :type Scene%20Component%20Object%20Reference))
  (Physics|SetSimulatePhysics (Variables|Default|GetBox) false)
  (Transformation|AttachComponentToComponent (VehicleSound|GetRootComponent) AttachTo "None" "KeepWorld" "KeepWorld" "KeepWorld" false))

(event EventDrop
  (Physics|SetSimulatePhysics (Variables|Default|GetBox) true)
  (Transformation|DetachFromActor "KeepWorld" "KeepWorld" "KeepWorld"))

(fn ConstructionScript)