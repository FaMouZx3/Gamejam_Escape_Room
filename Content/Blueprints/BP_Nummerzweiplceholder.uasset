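; BP_Nummerzweiplceholder is a VR-grabbable physics cube with a TextRender label that displays a number.
; The Zahl event converts the value it receives to text and writes it to the label.
; Pickup, called by BP_MotionController, disables cube physics and attaches the root component to the given component, keeping world transform.
; Drop re-enables physics and detaches the actor in place.
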(event Custom|Zahl
  (params (Zahl :type String))
  (Rendering|Components|TextRender|SetText (Variables|Default|GetTextRender) (Utilities|Text|ToText(String) Zahl)))

(event EventBeginPlay)

(event Collision|EventActorBeginOverlap
  (params (OtherActor :type Actor%20Object%20Reference)))

(event EventTick
  (params (DeltaSeconds :type Float%20%28single-precision%29)))

(event EventPickup
  (params (AttachTo :type Scene%20Component%20Object%20Reference))
  (Physics|SetSimulatePhysics (Variables|Default|GetCube) false)
  (Transformation|AttachComponentToComponent (VehicleSound|GetRootComponent) AttachTo "None" "KeepWorld" "KeepWorld" "KeepWorld" false))

(event EventDrop
  (Physics|SetSimulatePhysics (Variables|Default|GetCube) true)
  (Transformation|DetachFromActor "KeepWorld" "KeepWorld" "KeepWorld"))

(fn ConstructionScript)